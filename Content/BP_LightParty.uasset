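; BP_LightParty is a party light Blueprint that continuously randomizes the color of its PointLight.
; BeginPlay calls StartRandomLight, which plays a Timeline from the start and calls itself again when it finishes, forming an endless loop.
; Each Timeline update rolls new random red, green and blue values, scaled from zero by the Timeline alpha, so the color changes on every update.
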(event `self.ReceiveBeginPlay`
  (`self.StartRandomLight`))

(event `StartRandomLight`
  (bind (_direction _alpha) (`Timeline|Timeline` :!via `PlayFromStart`)
    (:`Update`
      (`LightComponent.SetLightColor` (`self.PointLight`) (make `LinearColor` (`KismetMathLibrary.Lerp` 0.0 (`KismetMathLibrary.RandomFloatInRange` 0.0 1.0) _alpha) (`KismetMathLibrary.Lerp` 0.0 (`KismetMathLibrary.RandomFloatInRange` 0.0 1.0) _alpha) (`KismetMathLibrary.Lerp` 0.0 (`KismetMathLibrary.RandomFloatInRange` 0.0 1.0) _alpha) 1.0) true))
    (:`Finished`
      (`self.StartRandomLight`))))

(fn `UserConstructionScript`)